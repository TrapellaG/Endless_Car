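; Floor tile actor for an endless vehicle course that randomly spawns either a blocker or a coin pickup.
; The construction script caches spawn-point transforms, then adds a child actor at a random one, usually a coin from one of two weighted branches.
; Overlapping the end trigger asks VehicleAdvGameMode to add another tile, then destroys this one after a delay.
; Side dead areas call SilentDeath on the vehicle, and GetAttachedTransform exposes the attach point.
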(event OnComponentBeginOverlap(EndTrigger)
  (params (OverlappedComponent :type Primitive%20Component%20Object%20Reference) (OtherActor :type Actor%20Object%20Reference) (OtherComp :type Primitive%20Component%20Object%20Reference) (OtherBodyIndex :type Integer) (bFromSweep :type Boolean) (SweepResult :type Hit%20Result%20Structure%20%28by%20ref%29))
  (bind _asvehicle_adv_game_mode (Utilities|Casting|CastToVehicleAdvGameMode (Game|GetGameMode)))
  (Default|AddFloorTile _asvehicle_adv_game_mode)
  (Utilities|FlowControl|Delay 2.0)
  (Actor|DestroyActor))

(event OnComponentBeginOverlap(DeadAreaRight)
  (params (OverlappedComponent :type Primitive%20Component%20Object%20Reference) (OtherActor :type Actor%20Object%20Reference) (OtherComp :type Primitive%20Component%20Object%20Reference) (OtherBodyIndex :type Integer) (bFromSweep :type Boolean) (SweepResult :type Hit%20Result%20Structure%20%28by%20ref%29))
  (bind _asvehicle_blueprint (Utilities|Casting|CastToVehicleBlueprint OtherActor))
  (Default|SilentDeath _asvehicle_blueprint))

(event OnComponentBeginOverlap(DeadAreaLeft)
  (params (OverlappedComponent :type Primitive%20Component%20Object%20Reference) (OtherActor :type Actor%20Object%20Reference) (OtherComp :type Primitive%20Component%20Object%20Reference) (OtherBodyIndex :type Integer) (bFromSweep :type Boolean) (SweepResult :type Hit%20Result%20Structure%20%28by%20ref%29))
  (bind _asvehicle_blueprint (Utilities|Casting|CastToVehicleBlueprint OtherActor))
  (Default|SilentDeath _asvehicle_blueprint))

(event EventBeginPlay)

(event Collision|EventActorBeginOverlap
  (params (OtherActor :type Actor%20Object%20Reference)))

(event EventTick
  (params (DeltaSeconds :type Float%20%28single-precision%29)))

(fn ConstructionScript
  (CallFunction|SetSpawnPoints)
  (switch int (Math|Random|RandomIntegerinRange 0 10)
    (:Default
      (CallFunction|SpawnCoins))
    (:0
      (CallFunction|SpawnBlocker))))

(fn GetAttachedTransform
  (return (Transformation|GetWorldTransform (Variables|Default|GetAttachPoint))))

(fn SetSpawnPoints
  (Variables|Default|SetSpawnPointsBlocks (Utilities|Array|MakeArray (Transformation|GetRelativeTransform (Variables|Default|GetSpawnPointR)) (Transformation|GetRelativeTransform (Variables|Default|GetSpawnPointL)) (Transformation|GetRelativeTransform (Variables|Default|GetSpawnPoint)) (Transformation|GetRelativeTransform (Variables|Default|GetSpawnPointMidL)) (Transformation|GetRelativeTransform (Variables|Default|GetSpawnPointMidR))))
  (Variables|Default|SetSpawnPointsCoins (Utilities|Array|MakeArray (Transformation|GetRelativeTransform (Variables|Default|GetCoinSpawn2)) (Transformation|GetRelativeTransform (Variables|Default|GetCoinSpawn3)) (Transformation|GetRelativeTransform (Variables|Default|GetCoinSpawn1)))))

(fn SpawnBlocker
  (bind _spawnpointsblocks (Variables|Default|GetSpawnPointsBlocks))
  (AddComponent|AddChildActorComponent false (Utilities|Array|Get(acopy) _spawnpointsblocks (Math|Random|RandomIntegerinRange 0 (Utilities|Array|LastIndex _spawnpointsblocks)))))

(fn SpawnCoins
  (bind _spawnpointscoins (Variables|Default|GetSpawnPointsCoins))
  (bind _returnvalue (Utilities|Array|LastIndex _spawnpointscoins))
  (bind _returnvalue_2 (Math|Random|RandomIntegerinRange 0 _returnvalue))
  (bind _output (Utilities|Array|Get(acopy) _spawnpointscoins _returnvalue_2))
  (if (Class|KismetMathLibrary|RandomBoolwithWeightfromStream 0.8 (Math|Random|MakeRandomStream (Math|Random|RandomIntegerinRange -10000 10000)))
    (AddComponent|AddChildActorComponent false _output)
    (else
      (AddComponent|AddChildActorComponent false _output))))